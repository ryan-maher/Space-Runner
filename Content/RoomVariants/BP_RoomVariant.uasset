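; Room tile for a first-person parkour runner, exposing an attach-point transform.
; Reaching the end trigger once has RunGameMode add a floor tile and increment score, then the room destroys itself after a delay.
; Back-frame hits kill the player when a forward-vector/hit-normal dot check passes, and a doorway volume briefly suppresses wall running.
; An overlap trigger slides both doors via timelines, with delayed resets to their starting positions.
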(event OnComponentBeginOverlap(EndTrigger)
  (params (OverlappedComponent :type Primitive%20Component%20Object%20Reference) (OtherActor :type Actor%20Object%20Reference) (OtherComp :type Primitive%20Component%20Object%20Reference) (OtherBodyIndex :type Integer) (bFromSweep :type Boolean) (SweepResult :type Hit%20Result%20Structure%20%28by%20ref%29))
  ;[1 1 1] Spawn new room variant and destroy old one
  (Utilities|Casting|CastToBP_FirstPersonCharacter OtherActor)
  (bind _asrun_game_mode (Utilities|Casting|CastToRunGameMode (Game|GetGameMode)))
  (Utilities|FlowControl|DoOnce false
    (:Completed
      (Default|AddFloorTile _asrun_game_mode)
      (Default|IncrementScore _asrun_game_mode)
      (Utilities|FlowControl|Delay 1.0)
      (Actor|DestroyActor))))

(event OnComponentHit(BackFrame)
  (params (HitComponent :type Primitive%20Component%20Object%20Reference) (OtherActor :type Actor%20Object%20Reference) (OtherComp :type Primitive%20Component%20Object%20Reference) (NormalImpulse :type Vector :default "0, 0, 0") (Hit :type Hit%20Result%20Structure%20%28by%20ref%29))
  ;[1 1 1] Kill Player on head-on wall collision
  (bind _asbp_first_person_character (Utilities|Casting|CastToBP_FirstPersonCharacter OtherActor))
  (if (Math|Float|NearlyEqual(Float) (Math|Vector|DotProduct (Transformation|GetActorForwardVector _asbp_first_person_character) (.normal Hit)) 1.0 0.1)
    (Default|Death _asbp_first_person_character)))

(event OnComponentBeginOverlap(PreventWallRunArea)
  (params (OverlappedComponent :type Primitive%20Component%20Object%20Reference) (OtherActor :type Actor%20Object%20Reference) (OtherComp :type Primitive%20Component%20Object%20Reference) (OtherBodyIndex :type Integer) (bFromSweep :type Boolean) (SweepResult :type Hit%20Result%20Structure%20%28by%20ref%29))
  ;[1 1 1] Prevent wall running on edges of doorway
  (bind _asbp_first_person_character (Utilities|Casting|CastToBP_FirstPersonCharacter OtherActor))
  (Default|SuppressWallRun (Variables|/Game/FirstPerson/Blueprints/BP_FirstPersonCharacter.BP_FirstPersonCharacter_C|GetParkourMovement _asbp_first_person_character) 0.2))

(event OnComponentBeginOverlap(OpenDoor)
  (params (OverlappedComponent :type Primitive%20Component%20Object%20Reference) (OtherActor :type Actor%20Object%20Reference) (OtherComp :type Primitive%20Component%20Object%20Reference) (OtherBodyIndex :type Integer) (bFromSweep :type Boolean) (SweepResult :type Hit%20Result%20Structure%20%28by%20ref%29))
  ;[1 1 1] Sliding Doors Functionality
  (Utilities|FlowControl|Sequence
    (:then_0
      (Variables|Default|SetInitialDoorPosLeft (Variables|/Script/Engine.SceneComponent|GetRelativeLocation (Variables|Default|GetSlidingDoorLeft)))
      (bind _newtrack_0 (Timeline|Timeline PlayFromStart)
        (:Update
          (Utilities|FlowControl|Delay 0.005)
          (Transformation|SetRelativeLocation (Variables|Default|GetSlidingDoorLeft) (Math|Vector|MakeVector (.x (Variables|Default|GetInitialDoorPosLeft)) (+ _newtrack_0 (.y (Variables|Default|GetInitialDoorPosLeft))) (.z (Variables|Default|GetInitialDoorPosLeft))) false false)
          (Utilities|FlowControl|Delay 1.0)
          (Transformation|SetRelativeLocation (Variables|Default|GetSlidingDoorLeft) (Variables|Default|GetInitialDoorPosLeft) false false))))
    (:then_1
      (Variables|Default|SetInitialDoorPosRight (Variables|/Script/Engine.SceneComponent|GetRelativeLocation (Variables|Default|GetSlidingDoorRight)))
      (bind _newtrack_0_2 (Timeline|Timeline_0 PlayFromStart)
        (:Update
          (Utilities|FlowControl|Delay 0.005)
          (Transformation|SetRelativeLocation (Variables|Default|GetSlidingDoorRight) (Math|Vector|MakeVector (.x (Variables|Default|GetInitialDoorPosRight)) (+ _newtrack_0_2 (.y (Variables|Default|GetInitialDoorPosRight))) (.z (Variables|Default|GetInitialDoorPosRight))) false false)
          (Utilities|FlowControl|Delay 1.0)
          (Transformation|SetRelativeLocation (Variables|Default|GetSlidingDoorRight) (Variables|Default|GetInitialDoorPosRight) false false))))))

(event EventBeginPlay)

(event Collision|EventActorBeginOverlap
  (params (OtherActor :type Actor%20Object%20Reference)))

(event EventTick
  (params (DeltaSeconds :type Float%20%28single-precision%29)))

(fn ConstructionScript)

(fn GetAttachTransform
  (return (Transformation|GetWorldTransform (Variables|Default|GetAttachPoint))))